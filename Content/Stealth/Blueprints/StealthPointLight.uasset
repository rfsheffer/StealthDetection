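; StealthPointLight is a light actor for a stealth system that tells stealth third-person characters when they are within its range.
; The construction script sizes a detection sphere from LightDetectionRadius.
; BeginPlay registers the light with characters already inside the sphere, while actor overlap events register and unregister it as they enter and leave.
; SomeFunction is a stub that always returns true.
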(event Collision|EventActorBeginOverlap
  (params (OtherActor :type Actor%20Object%20Reference))
  (bind _asstealth_third_person_character (Utilities|Casting|CastToStealthThirdPersonCharacter OtherActor))
  (Default|RegisterLocalLight _asstealth_third_person_character self))

(event Collision|EventActorEndOverlap
  (params (OtherActor :type Actor%20Object%20Reference))
  (bind _asstealth_third_person_character (Utilities|Casting|CastToStealthThirdPersonCharacter OtherActor))
  (Default|UnRegisterLocalLight _asstealth_third_person_character self))

(event EventBeginPlay
  (for _array_element (Collision|GetOverlappingActors (Variables|Default|GetSphere) "/Script/Engine.Actor" :!class /Script/Engine.PrimitiveComponent)
    (bind _asstealth_third_person_character (Utilities|Casting|CastToStealthThirdPersonCharacter _array_element))
    (Default|RegisterLocalLight _asstealth_third_person_character self)))

(fn ConstructionScript
  (Components|Sphere|SetSphereRadius (Variables|Default|GetSphere) (Variables|Stealth|GetLightDetectionRadius) true))

(fn SomeFunction
  (params (NewParam :type Boolean :default false))
  (return true))