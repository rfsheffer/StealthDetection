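; StealthSpotLight is a spot light that tells stealth characters when they are inside its detection area.
; The Construction Script stretches and offsets a Cone component to follow the light's attenuation radius, with LightDetectionSize setting its width.
; On BeginPlay it registers itself with StealthThirdPersonCharacters already overlapping the Cone.
; Actor overlap events then register or unregister it as a local light as characters enter and leave.
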(event Collision|EventActorBeginOverlap
  (params (OtherActor :type Actor%20Object%20Reference))
  (bind _asstealth_third_person_character (Utilities|Casting|CastToStealthThirdPersonCharacter OtherActor))
  (Default|RegisterLocalLight _asstealth_third_person_character self))

(event Collision|EventActorEndOverlap
  (params (OtherActor :type Actor%20Object%20Reference))
  (bind _asstealth_third_person_character (Utilities|Casting|CastToStealthThirdPersonCharacter OtherActor))
  (Default|UnRegisterLocalLight _asstealth_third_person_character self))

(event EventBeginPlay
  (for _array_element (Collision|GetOverlappingActors (Variables|Default|GetCone) "/Script/Engine.Actor" :!class /Script/Engine.PrimitiveComponent)
    (bind _asstealth_third_person_character (Utilities|Casting|CastToStealthThirdPersonCharacter _array_element))
    (Default|RegisterLocalLight _asstealth_third_person_character self)))

(fn ConstructionScript
  (bind _cone (Variables|Default|GetCone))
  (bind _lightdetectionsize (Variables|Stealth|GetLightDetectionSize))
  (bind _spotlightcomponent (Variables|Default|GetSpotLightComponent))
  (bind _attenuationradius (Variables|/Script/Engine.PointLightComponent|GetAttenuationRadius _spotlightcomponent))
  (bind _returnvalue (/ _attenuationradius 1.4e+02))
  (Transformation|SetRelativeScale3D _cone (Math|Vector|MakeVector _lightdetectionsize _lightdetectionsize _returnvalue))
  (Transformation|SetRelativeLocation _cone (Math|Vector|MakeVector (/ (* _returnvalue 1e+02) 2.0) 0.0 0.0) false false))